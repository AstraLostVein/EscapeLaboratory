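; BP_DoubleDoors is a sliding double door that opens when something enters its Box trigger and closes when it leaves.
; Two timelines, OpenDoor and OpenDoor2, slide Door1 and Door2 apart along local Y and reverse to close them.
; An Open flag guards against repeated triggers, and BeginPlay sets both timelines' play rate from SpeedRateDoor.
; Overlaps are not filtered by actor or counted, so any end overlap closes the doors.
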(event `self.ReceiveBeginPlay`
  (`TimelineComponent.SetPlayRate` (`self.OpenDoor2`) (`self.SpeedRateDoor`))
  (`TimelineComponent.SetPlayRate` (`self.OpenDoor`) (`self.SpeedRateDoor`)))

(event `self.Box.OnComponentBeginOverlap`
  (params (OverlappedComponent :type "PrimitiveComponent Object Reference") (OtherActor :type "Actor Object Reference") (OtherComp :type "PrimitiveComponent Object Reference") (OtherBodyIndex :type Integer) (bFromSweep :type Boolean) (SweepResult :type "HitResult Structure (by ref)"))
  ;[0.01938 0.01938 0.01938] Open and cloose door With overlap
  (if (not (`self.Open?`))
    (set `self.Open?` true)
    (`|ExecutionSequence`
      (:`then_0`
        (bind (_direction _newtrack_0) (`Timeline|OpenDoor` :!label _label)
          (:`Update`
            (`SceneComponent.K2_SetRelativeLocation` (`self.Door1`) (`KismetMathLibrary.MakeVector` 0.0 (`KismetMathLibrary.Lerp` -65.0 -155.0 _newtrack_0)) false false))))
      (:`then_1`
        (bind (_direction_2 _newtrack_0_2) (`Timeline|OpenDoor2` :!label _label_2)
          (:`Update`
            (`SceneComponent.K2_SetRelativeLocation` (`self.Door2`) (`KismetMathLibrary.MakeVector` 0.0 (`KismetMathLibrary.Lerp` 60.0 155.0 _newtrack_0_2)) false false)))))))

(event `self.Box.OnComponentEndOverlap`
  (params (OverlappedComponent :type "PrimitiveComponent Object Reference") (OtherActor :type "Actor Object Reference") (OtherComp :type "PrimitiveComponent Object Reference") (OtherBodyIndex :type Integer))
  ;[0.01938 0.01938 0.01938] Open and cloose door With overlap
  (if (`self.Open?`)
    (set `self.Open?` false)
    (`|ExecutionSequence`
      (:`then_0`
        (goto _label :!via `Reverse`))
      (:`then_1`
        (goto _label_2 :!via `Reverse`)))))

(fn `UserConstructionScript`)