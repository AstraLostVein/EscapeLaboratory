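; BP_DoorReel is a door that slides open when something enters its Box trigger and closes when the overlap ends.
; The OpenDoor timeline lerps the Doors component along local Y, playing forward on overlap and reversing on exit.
; An OpenDoors flag guards against repeated triggers, and SpeedRateDoor sets the timeline play rate on BeginPlay.
; The overlap events apply no filter on the overlapping actor.
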(event `self.ReceiveBeginPlay`
  (`TimelineComponent.SetPlayRate` (`self.OpenDoor`) (`self.SpeedRateDoor`)))

(event `self.Box.OnComponentBeginOverlap`
  (params (OverlappedComponent :type "PrimitiveComponent Object Reference") (OtherActor :type "Actor Object Reference") (OtherComp :type "PrimitiveComponent Object Reference") (OtherBodyIndex :type Integer) (bFromSweep :type Boolean) (SweepResult :type "HitResult Structure (by ref)"))
  (if (not (`self.OpenDoors?`))
    (set `self.OpenDoors?` true)
    (bind (_direction _glidex) (`Timeline|OpenDoor` :!label _label)
      (:`Update`
        (`SceneComponent.K2_SetRelativeLocation` (`self.Doors`) (`KismetMathLibrary.MakeVector` 0.0 (`KismetMathLibrary.Lerp` 0.0 110.0 _glidex)) false false)))))

(event `self.Box.OnComponentEndOverlap`
  (params (OverlappedComponent :type "PrimitiveComponent Object Reference") (OtherActor :type "Actor Object Reference") (OtherComp :type "PrimitiveComponent Object Reference") (OtherBodyIndex :type Integer))
  (if (`self.OpenDoors?`)
    (set `self.OpenDoors?` false)
    (goto _label :!via `Reverse`)))

(fn `UserConstructionScript`)